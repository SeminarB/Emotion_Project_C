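; Character Blueprint that runs a short scripted Japanese dialogue test on BeginPlay, shown through PrintString.
; It prints a greeting, then checks the 挨拶 (greeting) variable to choose a printed reply and raise or lower the Koukando (affection) value by assignment.
; It then asks a Pikachu-or-Eevee question and overwrites 質問テスト1 with a matching response, which is never printed.
; The construction script is empty.
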(event `self.ReceiveBeginPlay`
  (`KismetSystemLibrary.PrintString` "こんにちは！")
  (if (`KismetStringLibrary.EqualEqual_StrStr` (`self.挨拶`) "こんにちは！")
    (bind _output_get (set `self.挨拶` "今日もいい天気ですね"))
    (`KismetSystemLibrary.PrintString` _output_get)
    (set `self.koukando` 1.0)
    (else
      (bind _output_get_2 (set `self.挨拶` "挨拶も返せないんですね(笑)"))
      (`KismetSystemLibrary.PrintString` _output_get_2)
      (set `self.koukando` -1.0)))
  (`KismetSystemLibrary.PrintString` "ピカチュウとイーブイどっちが好き？")
  (if (`KismetStringLibrary.EqualEqual_StrStr` (`self.質問テスト1`) "ピカチュウ")
    (set `self.質問テスト1` "電気タイプが好きなんだ")
    (else
      (set `self.質問テスト1` "色々進化できるから悩んじゃうね"))))

(fn `UserConstructionScript`)