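; WalkChr is a character Blueprint that runs a small scripted dialogue test in Japanese on BeginPlay.
; It prints a greeting, then checks the 挨拶 variable, overwrites it with a reply and sets Koukando (affection) positive or negative.
; It then prints a Pikachu-or-Eevee question and overwrites 質問テスト1 based on its current value.
; Both branches read existing variable values without waiting for input, and the replies are stored but never printed.
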(event `self.ReceiveBeginPlay`
  (`KismetSystemLibrary.PrintString` "こんにちは！")
  (if (`KismetStringLibrary.EqualEqual_StrStr` (`self.挨拶`) "こんにちは！")
    (set `self.挨拶` "今日もいい天気ですね")
    (set `self.koukando` 1.0)
    (else
      (set `self.挨拶` "挨拶も返せないんですね(笑)")
      (set `self.koukando` -1.0)))
  (`KismetSystemLibrary.PrintString` "ピカチュウとイーブイどっちが好き？")
  (if (`KismetStringLibrary.EqualEqual_StrStr` (`self.質問テスト1`) "ピカチュウ")
    (set `self.質問テスト1` "電気タイプが好きなんだ")
    (else
      (set `self.質問テスト1` "色々進化できるから悩んじゃうね"))))

(fn `UserConstructionScript`)